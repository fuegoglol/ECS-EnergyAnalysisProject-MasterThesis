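; AI controller that flies a possessed BP_Spaceship along a canned, looping movement pattern.
; A vector timeline, given a random play rate at BeginPlay, feeds the ship's move and rotate inputs, firing whenever it finishes.
; A FlipFlop alternates forward and reverse playback on each StartMovements call.
; UnPossess calls StopMovement, leaving the timeline-stopping StopMovements event uncalled in this graph.
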(event Custom|StartMovements
  (bind _controlledspaceship (Variables|Default|GetControlledSpaceship))
  (Utilities|FlowControl|FlipFlop
    (:A
      (bind _input (Timeline|SpaceshipMovements PlayFromStart)
        (:Update
          (Class|Spaceship|InputMove _controlledspaceship (Math|Vector2D|MakeVector2D (.z _input) 0.0))
          (Class|Spaceship|InputRotate _controlledspaceship (Math|Vector2D|MakeVector2D (.x _input) (.y _input))))
        (:Finished
          (Class|Spaceship|InputFire (Variables|Default|GetControlledSpaceship))
          (CallFunction|StartMovements))))
    (:B
      (Timeline|SpaceshipMovements ReverseFromEnd))))

(event Custom|StopMovements
  (bind _controlledspaceship (Variables|Default|GetControlledSpaceship))
  (bind _input (Timeline|SpaceshipMovements Stop)
    (:Update
      (Class|Spaceship|InputMove _controlledspaceship (Math|Vector2D|MakeVector2D (.z _input) 0.0))
      (Class|Spaceship|InputRotate _controlledspaceship (Math|Vector2D|MakeVector2D (.x _input) (.y _input))))
    (:Finished
      (Class|Spaceship|InputFire (Variables|Default|GetControlledSpaceship))
      (CallFunction|StartMovements))))

(event EventBeginPlay
  (Components|Timeline|SetPlayRate (Variables|Default|GetSpaceshipMovements) (Math|Random|RandomFloatinRange 0.1 1.0)))

(event EventPossess
  (params (PossessedPawn :type Pawn%20Object%20Reference))
  (bind _asbp_spaceship (Utilities|Casting|CastToBP_Spaceship (Pawn|GetControlledPawn)))
  (Variables|Default|SetControlledSpaceship _asbp_spaceship)
  (CallFunction|StartMovements))

(event EventUnPossess
  (params (UnpossessedPawn :type Pawn%20Object%20Reference))
  (AI|Navigation|StopMovement))

(fn ConstructionScript)